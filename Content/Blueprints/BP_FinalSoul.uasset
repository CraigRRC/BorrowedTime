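; BP_FinalSoul is a soul pickup that adds game time and can ease the Grim Reaper's pursuit when the player touches it.
; On player overlap, it passes the reaper's SecondsTillBoost to the game mode's AddTime.
; If FollowDistance is at least MinFollowDistance plus DistanceBoost, it adds DistanceBoost to that distance and subtracts SpeedIncrease from FollowSpeed.
; Either way, it destroys itself after a short delay.
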(event OnComponentBeginOverlap(Collider)
  (params (OverlappedComponent :type Primitive%20Component%20Object%20Reference) (OtherActor :type Actor%20Object%20Reference) (OtherComp :type Primitive%20Component%20Object%20Reference) (OtherBodyIndex :type Integer) (bFromSweep :type Boolean) (SweepResult :type Hit%20Result%20Structure%20%28by%20ref%29))
  (bind _grim_reaper_ref (Variables|Default|GetGrim%20Reaper%20Ref))
  (bind _distance_boost (Variables|/Game/Denise/GrimReaper/BP_GrimReaper.BP_GrimReaper_C|GetDistance%20Boost _grim_reaper_ref))
  (if (== OtherActor (Variables|Default|GetPlayerReference))
    (Default|AddTime (Variables|Default|GetGameModeRef) (Variables|/Game/Denise/GrimReaper/BP_GrimReaper.BP_GrimReaper_C|GetSeconds%20Till%20Boost _grim_reaper_ref))
    (if (>= (Variables|/Game/Denise/GrimReaper/BP_GrimReaper.BP_GrimReaper_C|GetFollow%20Distance _grim_reaper_ref) (+ (Variables|/Game/Denise/GrimReaper/BP_GrimReaper.BP_GrimReaper_C|GetMin%20Follow%20distance _grim_reaper_ref) _distance_boost))
      (Variables|/Game/Denise/GrimReaper/BP_GrimReaper.BP_GrimReaper_C|SetFollow%20Distance _grim_reaper_ref (+ (Variables|/Game/Denise/GrimReaper/BP_GrimReaper.BP_GrimReaper_C|GetFollow%20Distance _grim_reaper_ref) _distance_boost))
      (Variables|/Game/Denise/GrimReaper/BP_GrimReaper.BP_GrimReaper_C|SetFollow%20Speed _grim_reaper_ref (- (Variables|/Game/Denise/GrimReaper/BP_GrimReaper.BP_GrimReaper_C|GetFollow%20Speed _grim_reaper_ref) (Variables|/Game/Denise/GrimReaper/BP_GrimReaper.BP_GrimReaper_C|GetSpeed%20Increase _grim_reaper_ref)))
      (Utilities|FlowControl|Delay 0.1)
      (Actor|DestroyActor)
      (else
        (Utilities|FlowControl|Delay 0.1)
        (Actor|DestroyActor)))))

(event EventBeginPlay
  ;[0.3804 0.8285 1] Set reference to player
  (bind _asbp_player (Utilities|Casting|CastToBP_Player (Game|Player|GetPlayerPawn 0)))
  (Variables|Default|SetPlayerReference _asbp_player)
  ;[1 1 1] Set reference to game mode
  (bind _asbp_game_mode (Utilities|Casting|CastToBP_GameMode (Game|GetGameMode)))
  (Variables|Default|SetGameModeRef _asbp_game_mode)
  (bind _returnvalue (Actor|GetActorOfClass "/Game/Denise/GrimReaper/BP_GrimReaper.BP_GrimReaper_C"))
  (Variables|Default|SetGrim%20Reaper%20Ref _returnvalue))

(fn ConstructionScript)