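; Player Blueprint that moves along world X by applying physics forces to its capsule, using Enhanced Input.
; BeginPlay adds the default mapping context; IA_Move applies acceleration-based force scaled by input and records the last direction.
; When input is canceled or completed, Tick applies braking force against that recorded direction until X velocity is near zero.
; Tick also prints X velocity, and the jump input event is empty.
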(event Input|EnhancedActionEvents|EnhancedInputActionIA_Move
  (params (ActionValue :type Float%20%28double-precision%29) (ElapsedSeconds :type Float%20%28double-precision%29) (TriggeredSeconds :type Float%20%28double-precision%29) (InputAction :type Input%20Action%20Object%20Reference :default "/Game/Input/IA_Move.IA_Move"))
  (:Triggered
    (Variables|Default|SetInputCanceled false)
    (Physics|AddForce (Variables|Default|GetCapsule) (Math|Vector|MakeVector (* ActionValue (Variables|Default|GetMovementForce)) 0.0 0.0) "None" true)
    (Variables|Default|SetLastTriggeredDirection ActionValue))
  (:Canceled
    (Variables|Default|SetInputCanceled true :!label _label))
  (:Completed
    (goto _label)))

(event Input|EnhancedActionEvents|EnhancedInputActionIA_Jump
  (params (ActionValue :type Boolean) (ElapsedSeconds :type Float%20%28double-precision%29) (TriggeredSeconds :type Float%20%28double-precision%29) (InputAction :type Input%20Action%20Object%20Reference :default "/Game/Input/IA_Jump.IA_Jump")))

(event EventBeginPlay
  (Input|AddMappingContext (PlayerController|LocalPlayerSubsystems|GetEnhancedInputLocalPlayerSubsystem (Game|GetPlayerController 0)) "/Game/Input/IMC_Default.IMC_Default" 0 "(bIgnoreAllPressedKeysUntilRelease=True,bForceImmediately=False,bNotifyUserSettings=False)"))

(event Collision|EventActorBeginOverlap
  (params (OtherActor :type Actor%20Object%20Reference)))

(event EventTick
  (params (DeltaSeconds :type Float%20%28single-precision%29))
  (Development|PrintString (Utilities|String|ToString(Float) (.x (Transformation|GetVelocity))))
  (if (Variables|Default|GetInputCanceled)
    (if (not (Math|Float|NearlyEqual(Float) (.x (Transformation|GetVelocity)) 0.0 5.0))
      (if (> (Variables|Default|GetLastTriggeredDirection) 0.0)
        (Physics|AddForce (Variables|Default|GetCapsule) (Math|Vector|MakeVector (* (Variables|Default|GetBraking%20Force) -1.0) 0.0 0.0) "None" true)
        (else
          (Physics|AddForce (Variables|Default|GetCapsule) (Math|Vector|MakeVector (Variables|Default|GetBraking%20Force) 0.0 0.0) "None" true))))))

(fn ConstructionScript)