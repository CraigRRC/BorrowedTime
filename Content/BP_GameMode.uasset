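; Game mode that runs a countdown and unleashes the Grim Reaper when time runs out.
; BeginPlay shows the timer widget and caches the reaper; Tick compares game time to MaxTime to update TimeLeft and GameRunning.
; Once over, Tick keeps printing game over and, after a short Delay, sets the reaper's follow distance to zero and changes its follow speed.
; AddTime extends the limit by raising MaxTime.
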(event EventBeginPlay
  (bind _returnvalue (UserInterface|CreateWidget "/Game/WBP_Timer.WBP_Timer_C"))
  (UserInterface|Viewport|AddtoViewport _returnvalue 0)
  (Variables|Default|SetCurrent%20Time (Utilities|Time|GetGameTimeinSeconds))
  (bind _returnvalue_2 (Actor|GetActorOfClass "/Game/Denise/GrimReaper/BP_GrimReaper.BP_GrimReaper_C"))
  (Variables|Default|SetGrim%20Reaper%20Ref _returnvalue_2))

(event EventTick
  (params (DeltaSeconds :type Float%20%28single-precision%29))
  (bind _grim_reaper_ref (Variables|Default|GetGrim%20Reaper%20Ref))
  (if (Variables|Default|GetGame%20Running)
    ;[0.3049 0.6566 1] Set Game running to true if current time is less than Max time and false if not
    (Variables|Default|SetGame%20Running (<= (Variables|Default|GetCurrent%20Time) (Variables|Default|GetMax%20Time)))
    (Variables|Default|SetCurrent%20Time (Utilities|Time|GetGameTimeinSeconds))
    (Variables|Default|SetTime%20Left (- (Variables|Default|GetMax%20Time) (Variables|Default|GetCurrent%20Time)))
    (else
      (Development|PrintString "GAME OVER")
      (Variables|Default|SetTime%20Left 0.0)
      (Utilities|FlowControl|Delay 1.0)
      (Variables|/Game/Denise/GrimReaper/BP_GrimReaper.BP_GrimReaper_C|SetFollow%20Distance _grim_reaper_ref 0.0)
      (Variables|/Game/Denise/GrimReaper/BP_GrimReaper.BP_GrimReaper_C|SetFollow%20Speed _grim_reaper_ref 4.5))))

(fn ConstructionScript)

(fn AddTime
  (params (TimeValue :type Float%20%28double-precision%29))
  (Variables|Default|SetMax%20Time (+ TimeValue (Variables|Default|GetMax%20Time)))
  (Development|PrintString "TIME ADDED" true true "(R=0.000000,G=0.660000,B=1.000000,A=1.000000)" 2.0 "TIMEADD"))