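; Player for side-on movement along X, driving a physics capsule with Enhanced Input for move, jump and a pause menu toggle.
; Capsule gravity doubles as the airborne flag: a downward sphere trace turns it off on landing, while jump release or a failed line trace plus coyote delay turns it on.
; Tick uses that state for braking, extra fall gravity, air control and speed caps, and turns the mesh toward travel direction.
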(event Input|EnhancedActionEvents|EnhancedInputActionIA_Move
  (params (ActionValue :type Float%20%28double-precision%29) (ElapsedSeconds :type Float%20%28double-precision%29) (TriggeredSeconds :type Float%20%28double-precision%29) (InputAction :type Input%20Action%20Object%20Reference :default "/Game/Input/IA_Move.IA_Move"))
  ;[0.1741 1 0.08618] Player
  ;;[1 1 1] Input
  (:Triggered
    (Variables|Default|SetbStopApplyingBrakingForce false)
    (Variables|Default|SetInputCanceled false)
    (Physics|AddForce (Variables|Default|GetCapsule) (Math|Vector|MakeVector (* ActionValue (Variables|Default|GetMovementForce)) 0.0 0.0) "None" true))
  (:Canceled
    (Variables|Default|SetInputCanceled true :!label _label))
  (:Completed
    (goto _label)))

(event Input|EnhancedActionEvents|EnhancedInputActionIA_Jump
  (params (ActionValue :type Boolean) (ElapsedSeconds :type Float%20%28double-precision%29) (TriggeredSeconds :type Float%20%28double-precision%29) (InputAction :type Input%20Action%20Object%20Reference :default "/Game/Input/IA_Jump.IA_Jump"))
  ;[0.1741 1 0.08618] Player
  ;;[1 1 1] Input
  (:Triggered
    (if (not (Class|PrimitiveComponent|IsGravityEnabled (Variables|Default|GetCapsule)))
      (Physics|AddImpulse (Variables|Default|GetCapsule) (Math|Vector|MakeVector 0.0 0.0 (Variables|Default|GetJumpForce)) "None" true)))
  (:Completed
    (Physics|SetEnableGravity (Variables|Default|GetCapsule) true)))

(event Input|EnhancedActionEvents|EnhancedInputActionIA_Pause
  (params (ActionValue :type Boolean) (ElapsedSeconds :type Float%20%28double-precision%29) (TriggeredSeconds :type Float%20%28double-precision%29) (InputAction :type Input%20Action%20Object%20Reference :default "/Game/Input/IA_Pause.IA_Pause"))
  ;[0.1741 1 0.08618] Player
  ;;[1 1 1] Input
  (if (Game|IsGamePaused)
    (Game|SetGamePaused false)
    (Utilities|IsValid (Variables|Default|GetPauseWidget)
      (:Is%20Valid
        (Widget|RemovefromParent (Variables|Default|GetPauseWidget))))
    (else
      (Game|SetGamePaused true)
      (bind _returnvalue (UserInterface|CreateWidget "/Game/Denise/Menu/W_PauseMenu.W_PauseMenu_C"))
      (bind _output_get (Variables|Default|SetPauseWidget _returnvalue))
      (UserInterface|Viewport|AddtoPlayerScreen _output_get))))

(event EventBeginPlay
  ;[0.1741 1 0.08618] Player
  ;;[1 1 1] Initalize
  (Input|AddMappingContext (PlayerController|LocalPlayerSubsystems|GetEnhancedInputLocalPlayerSubsystem (Game|GetPlayerController 0)) "/Game/Input/IMC_Default.IMC_Default" 0 "(bIgnoreAllPressedKeysUntilRelease=True,bForceImmediately=False,bNotifyUserSettings=False)"))

(event EventTick
  (params (DeltaSeconds :type Float%20%28single-precision%29))
  (bind _returnvalue (Transformation|GetVelocity))
  (bind _returnvalue_2 (Transformation|GetVelocity))
  (bind _returnvalue_3 (Transformation|GetVelocity))
  (bind _returnvalue_4 (Transformation|GetVelocity))
  (bind _returnvalue_5 (Transformation|GetVelocity))
  (bind _returnvalue_6 (Transformation|GetVelocity))
  (bind _returnvalue_7 (Transformation|GetVelocity))
  (bind _returnvalue_8 (Transformation|GetVelocity))
  (bind _returnvalue_9 (Utilities|Time|GetWorldDeltaSeconds))
  (bind _returnvalue_10 (Transformation|GetVelocity))
  (bind _maxairvelocity (Variables|Default|GetMaxAirVelocity))
  (bind _maxgroundvelocity (Variables|Default|GetMaxGroundVelocity))
  (bind _rotationspeed (Variables|Default|GetRotationSpeed))
  (bind _returnvalue_11 (* _maxairvelocity -1.0))
  (bind _returnvalue_12 (* _maxgroundvelocity -1.0))
  ;[0.1741 1 0.08618] Player
  (Utilities|FlowControl|Sequence
    (:then_0
      ;;[1 1 1] Braking
      (if (not (Class|PrimitiveComponent|IsGravityEnabled (Variables|Default|GetCapsule)))
        (if (Variables|Default|GetInputCanceled)
          (if (Math|Float|NearlyEqual(Float) (.x (Transformation|GetVelocity)) 0.0 5.0)
            (Physics|SetPhysicsLinearVelocity (Variables|Default|GetCapsule) "0, 0, 0" false "None")
            (elif (> (.x (Transformation|GetVelocity)) 0.0)
              (if (not (Variables|Default|GetbStopApplyingBrakingForce))
                (Physics|AddForce (Variables|Default|GetCapsule) (Math|Vector|MakeVector (* (Variables|Default|GetBraking%20Force) -1.0) 0.0 0.0) "None" true)
                (if (and (<= (.x _returnvalue_7) 1e+02) (>= (.x _returnvalue_7) 0.0))
                  (Variables|Default|SetbStopApplyingBrakingForce true :!label _label)))
              (elif (not (Variables|Default|GetbStopApplyingBrakingForce))
                (Physics|AddForce (Variables|Default|GetCapsule) (Math|Vector|MakeVector (Variables|Default|GetBraking%20Force) 0.0 0.0) "None" true)
                (if (and (<= (.x _returnvalue_8) 0.0) (>= (.x _returnvalue_8) -1e+02))
                  (goto _label))))))))
    (:then_1
      ;;[1 1 1] GroundCheck
      (if (Class|PrimitiveComponent|IsGravityEnabled (Variables|Default|GetCapsule))
        (bind (_outhit _returnvalue_13) (Collision|SphereTraceByChannel (Transformation|GetActorLocation) (+ (Transformation|GetActorLocation) (* (Transformation|GetActorUpVector) -8e+01)) 2e+01 "TraceTypeQuery1" false 0 "None"))
        (Variables|Default|SetGroundHit _outhit)
        (if _returnvalue_13
          (Physics|SetEnableGravity (Variables|Default|GetCapsule) false)
          (Class|PrimitiveComponent|SetAllPhysicsLinearVelocity (Variables|Default|GetCapsule) (Math|Vector|MakeVector (.x (Transformation|GetVelocity)) 0.0 0.0) false))))
    (:then_2
      (Utilities|FlowControl|Sequence
        (:then_1
          ;;[1 1 1] FallCheck
          (if (Class|PrimitiveComponent|IsGravityEnabled (Variables|Default|GetCapsule))
            (Physics|AddForce (Variables|Default|GetCapsule) (Math|Vector|MakeVector 0.0 0.0 (Variables|Default|GetAdditionalGravity)) "None" true)
            (Variables|Default|SetMovementForce (Variables|Default|GetAirControl))
            (else
              (Variables|Default|SetMovementForce 4e+03)
              (bind (_outhit_2 _returnvalue_14) (Collision|LineTraceByChannel (Transformation|GetActorLocation) (+ (Transformation|GetActorLocation) (* (Transformation|GetActorUpVector) -1.5e+02)) "TraceTypeQuery1" false 0 "None"))
              (Variables|Default|SetFallCheck _outhit_2)
              (if _returnvalue_14
                (Variables|Default|SetbShouldFall false)
                (else
                  (Variables|Default|SetbShouldFall true))))))))
    (:then_3
      ;;[1 1 1] CoyoteTime
      (if (Variables|Default|GetbShouldFall)
        (Utilities|FlowControl|Delay (Variables|Default|GetCoyoteTime))
        (Physics|SetEnableGravity (Variables|Default|GetCapsule) true)))
    (:then_4
      ;;[1 1 1] AirControl/Landing
      (if (Class|PrimitiveComponent|IsGravityEnabled (Variables|Default|GetCapsule))
        (if (>= (.x _returnvalue_4) (Variables|Default|GetMaxAirVelocity))
          (Physics|SetPhysicsLinearVelocity (Variables|Default|GetCapsule) (Math|Vector|MakeVector (Variables|Default|GetMaxAirVelocity) (.y _returnvalue_6) (.z _returnvalue_6)) false "None")
          (elif (<= (.x _returnvalue_4) _returnvalue_11)
            (Physics|SetPhysicsLinearVelocity (Variables|Default|GetCapsule) (Math|Vector|MakeVector _returnvalue_11 (.y _returnvalue_5) (.z _returnvalue_5)) false "None")))
        (elif (>= (.x _returnvalue) (Variables|Default|GetMaxGroundVelocity))
          (Physics|SetPhysicsLinearVelocity (Variables|Default|GetCapsule) (Math|Vector|MakeVector (Variables|Default|GetMaxGroundVelocity) (.y _returnvalue_3) (.z _returnvalue_3)) false "None")
          (elif (<= (.x _returnvalue) _returnvalue_12)
            (Physics|SetPhysicsLinearVelocity (Variables|Default|GetCapsule) (Math|Vector|MakeVector _returnvalue_12 (.y _returnvalue_2) (.z _returnvalue_2)) false "None")))))
    (:then_5
      ;;[1 1 1] Pump the brakes
      (if (Variables|Default|GetbStopApplyingBrakingForce)
        (Physics|SetPhysicsLinearVelocity (Variables|Default|GetCapsule) (Math|Vector|MakeVector 0.0 (.y _returnvalue_10) (.z _returnvalue_10)) false "None")))
    (:then_6
      ;;[1 1 1] Character rotation
      ;;;[1 1 1] If the character isn't moving, don't rotate back to original state.
      (if (!= (Math|Vector|VectorLengthXY (Transformation|GetVelocity)) 0.0)
        (if (< (.x (Transformation|GetVelocity)) 0.0)
          (Transformation|SetRelativeRotation (Variables|Default|GetPlayerMesh) (Math|Interpolation|RInterpTo (Variables|/Script/Engine.SceneComponent|GetRelativeRotation (Variables|Default|GetPlayerMesh)) "0.000000,90.000000,0.000000" _returnvalue_9 _rotationspeed) false false)
          (Variables|Default|SetbCharacterFacingRight false)
          (else
            (Transformation|SetRelativeRotation (Variables|Default|GetPlayerMesh) (Math|Interpolation|RInterpTo (Variables|/Script/Engine.SceneComponent|GetRelativeRotation (Variables|Default|GetPlayerMesh)) "0.000000,-90.000000,0.000000" _returnvalue_9 _rotationspeed) false false)
            (Variables|Default|SetbCharacterFacingRight true)))))))

(fn ConstructionScript)