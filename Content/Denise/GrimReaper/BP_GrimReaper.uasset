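; Grim Reaper actor that pursues the player on the X/Z plane, with Y locked to the player's starting depth.
; Each Tick, FollowPlayer eases X and Z with FInterpTo toward targets from SetPos, scaled by FollowSpeed.
; SetPos targets FollowDistance behind the player when trailing by more than that on the positive axis, otherwise the player's exact position, despite its "Don't move at all" comment.
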(event EventBeginPlay
  (Utilities|FlowControl|Sequence
    (:then_0
      (bind _asbp_player (Utilities|Casting|CastToBP_Player (Game|Player|GetPlayerPawn 0)))
      (bind _output_get (Variables|Default|SetPlayer%20Ref _asbp_player))
      (Variables|Default|SetY%20Pos (.y (Transformation|GetActorLocation _output_get))))
    (:then_1
      (Transformation|SetActorLocation (Math|Vector|MakeVector (Variables|Default|GetX%20Pos) (Variables|Default|GetY%20Pos) (+ (Variables|Default|GetZ%20Pos) (Variables|Default|GetFollow%20Distance))) false false))))

(event EventTick
  (params (DeltaSeconds :type Float%20%28single-precision%29))
  (CallFunction|FollowPlayer DeltaSeconds))

(fn ConstructionScript)

(fn FollowPlayer
  (params (Delta%20Time :type Float%20%28double-precision%29))
  (bind _returnvalue (Transformation|GetActorLocation))
  (bind _follow_speed (Variables|Default|GetFollow%20Speed))
  (bind _player_ref (Variables|Default|GetPlayer%20Ref))
  (bind _returnvalue_2 (Transformation|GetActorLocation _player_ref))
  (bind _new_pos (CallFunction|SetPos (.x _returnvalue_2) (.x _returnvalue)))
  (bind _output_get (Variables|Default|SetX%20Pos (Math|Interpolation|FInterpTo (Variables|Default|GetX%20Pos) _new_pos Delta%20Time _follow_speed)))
  (bind _new_pos_2 (CallFunction|SetPos (.z _returnvalue_2) (.z _returnvalue)))
  (bind _output_get_2 (Variables|Default|SetZ%20Pos (Math|Interpolation|FInterpTo (Variables|Default|GetZ%20Pos) _new_pos_2 Delta%20Time _follow_speed)))
  (Transformation|SetActorLocation (Math|Vector|MakeVector _output_get (Variables|Default|GetY%20Pos) _output_get_2) false false))

(fn SetPos
  (params (PlayerPosition :type Float%20%28double-precision%29) (Reaper%20Pos :type Float%20%28double-precision%29))
  (bind _follow_distance (Variables|Default|GetFollow%20Distance))
  (bind _returnvalue (- PlayerPosition _follow_distance))
  (if (> _returnvalue Reaper%20Pos)
    ;[1 1 1] Move up
    (return _returnvalue)
    (else
      ;[1 1 1] Don't move at all
      (return PlayerPosition))))